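; BP_BaseItem is a clickable item actor that the player can pick up into an inventory.
; On click it casts the player character to Player1, checks that it is within a fixed distance, and passes its ItemInfo struct to AddItemToInventory.
; The actor destroys itself only when that call succeeds.
; The construction script rebuilds ItemInfo with the actor's own class, so the stored data records which class the item came from.
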(event MouseInput|EventActorOnClicked
  (params (ButtonPressed :type Key%20Structure :default "AnyKey"))
  (bind _asplayer_1 (Utilities|Casting|CastToPlayer1 (Game|GetPlayerCharacter 0)))
  (Math|Float|CompareFloat (Transformation|GetDistanceTo _asplayer_1) 4e+02
    (:<
      (bind _wasitemadded (Default|AddItemtoInventory _asplayer_1 (Variables|Default|GetItemInfo)))
      (if _wasitemadded
        (Actor|DestroyActor)))))

(fn ConstructionScript
  (|CallParentFunction)
  (Variables|Default|SetItemInfo (Utilities|Struct|MakeFItemInfo (.itemtype (Variables|Default|GetItemInfo)) (.itemname (Variables|Default|GetItemInfo)) (.itemimage (Variables|Default|GetItemInfo)) (Utilities|GetClass self) (.itemposition (Variables|Default|GetItemInfo)) (.itemprice (Variables|Default|GetItemInfo)) (.itemrarity (Variables|Default|GetItemInfo)) (.itemmainstat (Variables|Default|GetItemInfo)))))